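; Mine actor that explodes when any actor other than the grenade overlaps it.
; On overlap it activates its particle system, plays an explosion sound at the world origin rather than its own location, and destroys its StaticMesh and Cylinder components.
; The actor destroys itself after a delay, and no damage is applied in this Blueprint.
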(event `self.ReceiveActorBeginOverlap`
  (params (OtherActor :type "Actor Object Reference"))
  (if (not (== OtherActor "/Game/FirstPersonBP/Blueprints/PlayerStuff/Grenade.Grenade"))
    (`ActorComponent.Activate` (`self.ParticleSystem`) false)
    (`GameplayStatics.PlaySoundAtLocation` "/Game/StarterContent/Audio/Explosion02.Explosion02" (0.0 0.0 0.0))
    (`ActorComponent.K2_DestroyComponent` (`self.StaticMesh`))
    (`ActorComponent.K2_DestroyComponent` (`self.Cylinder`))
    (`KismetSystemLibrary.Delay` 7.0)
    (`self.K2_DestroyActor`)))

(fn `UserConstructionScript`)