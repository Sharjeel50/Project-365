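; Enemy character AI that wanders to random navigable points and runs at the player when it sees them or gets shot.
; Projectile hits on the capsule or head sphere reduce Health, with headshots dealing full damage, and Tick polls for death and wandering.
; Detonated grenades, mines or an EnemyExploded call launch it upward before death.
; Death plays an animation, enables physics, sprays blood particles that spawn randomized decals, then destroys the actor.
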(event `OnParticleCollide_Event_0`
  (params (EventName :type Name) (EmitterTime :type "Float (double-precision)") (ParticleTime :type Integer) (Location :type "Vector Structure") (Velocity :type "Vector Structure") (Direction :type "Vector Structure") (Normal :type "Vector Structure") (BoneName :type Name) (PhysMat :type "PhysicalMaterial Object Reference"))
  ;[1 1 1] Blood decal
  (bind _returnvalue (`KismetMaterialLibrary.CreateDynamicMaterialInstance` "/Game/MaterialsAndTextures/Blood_Decal_M.Blood_Decal_M"))
  (`MaterialInstanceDynamic.SetScalarParameterValue` _returnvalue "Frame" (`KismetMathLibrary.Conv_IntToDouble` (`KismetMathLibrary.RandomInteger` 100)))
  (`GameplayStatics.SpawnDecalAtLocation` _returnvalue (`KismetMathLibrary.Conv_DoubleToVector` (`KismetMathLibrary.RandomFloatInRange` 30.0 75.0)) Location (`KismetMathLibrary.Conv_VectorToRotator` Normal) 30.0))

(event `self.ReceiveActorBeginOverlap`
  (params (OtherActor :type "Actor Object Reference"))
  ;[1 1 1] Explosives sensor
  (`|ExecutionSequence`
    (:`then_0`
      (bind _asgrenade (cast `/Game/FirstPersonBP/Blueprints/PlayerStuff/Grenade` OtherActor))
      (if (`/Game/FirstPersonBP/Blueprints/PlayerStuff/Grenade.IsDetonated` _asgrenade)
        (`self.LaunchCharacter` self (0.0 0.0 1000.0) false true :!label _label)
        (`KismetSystemLibrary.Delay` 0.2)
        (`KismetSystemLibrary.PrintText` "                                                                                                                              +Enemy Exploded!" true false (struct :`R` 1.0 :`A` 1.0) 5.0)
        ;[1 1 1] Death Sequence
        (bind _returnvalue (`GameplayStatics.SpawnEmitterAtLocation` "/Game/Particles/BloodSplatter_Particle.BloodSplatter_Particle" (`self.K2_GetActorLocation`) (struct) (2.0 2.0 2.0) :!label _label_2))
        (add `ParticleSystemComponent.OnParticleCollide` _returnvalue (delegate `OnParticleCollide_Event_0`))
        (`SkeletalMeshComponent.PlayAnimation` (`self.Mesh`) "/Game/Enemy/Animation/death_from_the_back.death_from_the_back" false)
        (`PrimitiveComponent.SetSimulatePhysics` (`self.Mesh`) true)
        (`PrimitiveComponent.SetSimulatePhysics` (`self.SkeletalMesh`) true)
        (`ActorComponent.K2_DestroyComponent` (`self.Capsule`))
        (`ActorComponent.K2_DestroyComponent` (`self.Sphere`))
        (`ActorComponent.K2_DestroyComponent` (`self.CapsuleComponent`))
        (`ActorComponent.K2_DestroyComponent` (`self.PawnSensing`))
        (`KismetSystemLibrary.Delay` 3.2)
        (`self.K2_DestroyActor`)))
    (:`then_1`
      (bind _asmine (cast `/Game/Blueprints/Mine` OtherActor))
      (set `self.ReferenceMine` _asmine)
      (goto _label))))

(event `Enemy Exploded`
  ;[1 1 1] Explosives sensor
  (goto _label))

(event `Enemy Died`
  ;[1 1 1] Death Sequence
  (if (<= (`self.Health`) 0.0)
    (`/Engine/EditorBlueprintResources/StandardMacros.DoOnce` false
      (:`Completed`
        (`KismetSystemLibrary.PrintText` "                                                                                                                              +Enemy Died!" true false (struct :`R` 1.0 :`B` 0.075397 :`A` 1.0) 5.0)
        (goto _label_2)))))

(event `self.Capsule.OnComponentHit`
  (params (HitComponent :type "PrimitiveComponent Object Reference") (OtherActor :type "Actor Object Reference") (OtherComp :type "PrimitiveComponent Object Reference") (NormalImpulse :type "Vector Structure") (Hit :type "HitResult Structure (by ref)"))
  ;[1 1 1] Gun hit
  (cast `/Game/FirstPersonBP/Blueprints/PlayerStuff/FirstPersonProjectile` OtherActor)
  (set `CharacterMovementComponent.MaxWalkSpeed` 625.0 (`self.CharacterMovement`))
  (set `self.In Range` true)
  (bind _asfirst_person_character (cast `/Game/FirstPersonBP/Blueprints/FirstPersonCharacter` (`GameplayStatics.GetPlayerCharacter` 0)))
  (`|AIMoveTo` self (0.0 0.0 0.0) _asfirst_person_character 10.0
    (:`then`
      (set `self.Health` (`KismetMathLibrary.FClamp` (- (`self.Health`) 10.0) 0.0 100.0))
      (bind _returnvalue (`GameplayStatics.SpawnEmitterAtLocation` "/Game/Particles/BloodSplatter_Particle.BloodSplatter_Particle" (`self.K2_GetActorLocation`) (struct) (2.0 2.0 2.0)))
      (add `ParticleSystemComponent.OnParticleCollide` _returnvalue (delegate `OnParticleCollide_Event_0`)))
    (:`OnSuccess`
      (`KismetSystemLibrary.Delay` 10.0 :!label _label_3)
      (set `self.In Range` false))
    (:`OnFail`
      (goto _label_3))))

(event `self.PawnSensing.OnSeePawn`
  (params (Pawn :type "Pawn Object Reference"))
  ;[1 1 1] Run Towards Player
  (set `CharacterMovementComponent.MaxWalkSpeed` 625.0 (`self.CharacterMovement`))
  (set `self.In Range` true)
  (bind _asfirst_person_character (cast `/Game/FirstPersonBP/Blueprints/FirstPersonCharacter` Pawn))
  (`|AIMoveTo` self (0.0 0.0 0.0) _asfirst_person_character 10.0
    (:`OnSuccess`
      _)
    (:`OnFail`
      _))
  (`KismetSystemLibrary.Delay` 10.0)
  (set `self.In Range` false))

(event `self.Sphere.OnComponentHit`
  (params (HitComponent :type "PrimitiveComponent Object Reference") (OtherActor :type "Actor Object Reference") (OtherComp :type "PrimitiveComponent Object Reference") (NormalImpulse :type "Vector Structure") (Hit :type "HitResult Structure (by ref)"))
  ;[1 1 1] Headshot
  (cast `/Game/FirstPersonBP/Blueprints/PlayerStuff/FirstPersonProjectile` OtherActor)
  (`ActorComponent.Activate` (`self.HeadShot_SoundFX`) true)
  (set `self.In Range` true)
  (bind _asfirst_person_character (cast `/Game/FirstPersonBP/Blueprints/FirstPersonCharacter` (`GameplayStatics.GetPlayerCharacter` 0)))
  (`|AIMoveTo` self (0.0 0.0 0.0) _asfirst_person_character
    (:`then`
      (set `self.Health` (`KismetMathLibrary.FClamp` (- (`self.Health`) 100.0) 0.0 100.0)))
    (:`OnSuccess`
      (`KismetSystemLibrary.Delay` 1.0 :!label _label_4)
      (set `self.In Range` false))
    (:`OnFail`
      (goto _label_4))))

(event `self.ReceiveTick`
  (params (DeltaSeconds :type "Float (single-precision)"))
  ;[1 1 1] Tick
  (`self.Enemy Died`)
  (`self.Find Player`))

(event `Find Player`
  ;[1 1 1] Find Player
  (if (`self.In Range`)
    _
    (elif (not (`self.Moving`))
      (`KismetSystemLibrary.Delay` 0.25)
      (`|AIMoveTo` self (`NavigationSystem.K2_GetRandomLocationInNavigableRadius` (`self.K2_GetActorLocation`) 4000.0) null 500.0
        (:`then`
          (set `self.Moving` true))
        (:`OnSuccess`
          (set `self.Moving` false :!label _label_5))
        (:`OnFail`
          (goto _label_5))))))

(fn `UserConstructionScript`)